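; Base gameplay ability that plays a montage and spawns a projectile carrying gameplay effects.
; After committing, it waits for Event.Montage events and builds an effect container spec from each received tag and data.
; If that spec has effects, it spawns ProjectileClass at the avatar's location and rotation, passing the spec and the avatar pawn as instigator.
; The ability ends when the montage blends out, is interrupted or is cancelled.
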(event `self.K2_ActivateAbility`
  (bind _returnvalue (`self.GetAvatarActorFromActorInfo`))
  (bind _returnvalue_2 (`self.K2_CommitAbility`))
  (if _returnvalue_2
    (bind (_asynctaskproxy _eventtag _eventdata) (`KayAbilityTask_PlayMontageAndWaitForEvent.PlayMontageAndWaitForEvent` "None" (`self.MontageToPlay`) (struct :`GameplayTags` (struct :`(TagName` "Event.Montage"))))
      (:`OnBlendOut`
        (`self.K2_EndAbility` :!label _label))
      (:`OnInterrupted`
        (goto _label))
      (:`OnCancelled`
        (goto _label))
      (:`EventReceived`
        (bind _returnvalue_3 (`self.MakeEffectContainerSpec` _eventtag _eventdata))
        (if (`KayBlueprintFunctionLibrary.DoesEffectContainerSpecHaveEffects` _returnvalue_3)
          (bind _aspawn (cast `Pawn` _returnvalue))
          (`|SpawnActorFromClass` (`self.ProjectileClass`) (`KismetMathLibrary.MakeTransform` (`Actor.K2_GetActorLocation` _returnvalue) (`Actor.K2_GetActorRotation` _returnvalue)) "Undefined" "OverrideRootScale" null _returnvalue_3 _aspawn))))))