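; BP_KayPlayerController is the player controller that owns the on-screen HUD for the Kay character.
; On possess, it creates the WB_HUD_PC widget if missing, adds it to the viewport, refreshes its icons and shows it.
; It then casts the pawn to BP_KayTest, caches it and pushes its health percentage to the HUD.
; A helper toggles HUD visibility between SelfHitTestInvisible and Hidden.
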(event `self.ReceiveBeginPlay`)

(event `self.ReceivePossess`
  (params (PossessedPawn :type "Pawn Object Reference"))
  (`|ExecutionSequence`
    (:`then_0`
      (`self.CreateHUD`))
    (:`then_1`
      (bind _asbp_kay_test (cast `/Game/Dungeon/Core/Characters/BP_KayTest` PossessedPawn))
      (set `self.As BP Kay Test` _asbp_kay_test)
      (`self.UpdateHUDInfo`))))

(fn `CreateHUD`
  (`/Engine/EditorBlueprintResources/StandardMacros.IsValid` (`self.OnScreenControls`)
    (:`Is Valid`
      _)
    (:`Is Not Valid`
      (bind _returnvalue (`|CreateWidget` "/Game/Dungeon/WB/WB_HUD_PC.WB_HUD_PC_C" self))
      (bind _output_get (set `self.OnScreenControls` _returnvalue))
      (`UserWidget.AddToViewport` _output_get 0)
      (message `/Game/Dungeon/WB/IHUD.UpdateIcons` (`self.OnScreenControls`))))
  (`self.ShowHUD` true))

(fn `ShowHUD`
  (params (Visible :type Boolean))
  (bind _onscreencontrols (`self.OnScreenControls`))
  (`/Engine/EditorBlueprintResources/StandardMacros.IsValid` _onscreencontrols
    (:`Is Valid`
      (`Widget.SetVisibility` _onscreencontrols (select `bool` Visible :`false` "Hidden" :`true` "SelfHitTestInvisible" :!type "ESlateVisibility Enum")))))

(fn `UpdateHUDInfo`
  (bind _onscreencontrols (`self.OnScreenControls`))
  (bind _percent (`/Game/Dungeon/Core/Characters/BP_KayTest.GetHealthInPercent` (`self.As BP Kay Test`)))
  (`/Engine/EditorBlueprintResources/StandardMacros.IsValid` _onscreencontrols
    (:`Is Valid`
      (message `/Game/Dungeon/WB/IHUD.SetHP` _onscreencontrols _percent))
    (:`Is Not Valid`
      (`KismetSystemLibrary.PrintString` "OnScreenControls   error"))))

(fn `UserConstructionScript`)