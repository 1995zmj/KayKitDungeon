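; BP_KayTest is a player character that equips a data-driven weapon and uses Gameplay Ability System abilities.
; On BeginPlay, if weapon data is valid, it attaches the weapon actor to the right-hand socket and grants weapon and skill abilities.
; Left and right mouse buttons activate those abilities, and possession caches the Kay player controller.
; Health and mana events call empty bar updates; GetHealthInPercent only prints values and returns zero.
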(event `self.ReceiveBeginPlay`
  (bind _weaponassetdata (`self.WeaponAssetData`))
  (`parent.ReceiveBeginPlay`)
  (`/Engine/EditorBlueprintResources/StandardMacros.IsValid` _weaponassetdata
    (:`Is Valid`
      (`|ExecutionSequence`
        (:`then_0`
          (bind _returnvalue (`|SpawnActorFromClass` (`KayDataAsset_Weapon.WeaponActor` _weaponassetdata) (`self.Spawn Transform`) "Undefined" "OverrideRootScale" null null))
          (bind _output_get (set `self.CurrentWeapon` _returnvalue))
          (`self.K2_AttachToComponent` _output_get (`self.Mesh`) "HandRightSocket" "KeepRelative" "KeepRelative" "KeepRelative" true))
        (:`then_1`
          (`self.GiveAbility` (`KayDataAsset.GrantedAbility` _weaponassetdata)))
        (:`then_2`
          (`self.GiveAbility` (`KayDataAsset.GrantedAbility` (`self.SkillAssetData`))))))))

(event `Key|RightMouseButton`
  (params (Key :type "Key Structure"))
  (:`Pressed`
    (`AbilitySystemComponent.TryActivateAbilityByClass` (`self.AbilitySystemComponent`) (`KayDataAsset.GrantedAbility` (`self.SkillAssetData`)) true)))

(event `Key|LeftMouseButton`
  (params (Key :type "Key Structure"))
  (:`Pressed`
    (`AbilitySystemComponent.TryActivateAbilityByClass` (`self.AbilitySystemComponent`) (`KayDataAsset.GrantedAbility` (`self.WeaponAssetData`)) true)))

(event `self.ReceivePossessed`
  (params (NewController :type "Controller Object Reference"))
  (bind _asbp_kay_player_controller (cast `/Game/Dungeon/Core/Characters/BP_KayPlayerController` NewController))
  (set `self.BP Kay Player Controller` _asbp_kay_player_controller))

(event `self.ReceiveUnpossessed`
  (params (OldController :type "Controller Object Reference"))
  (set `self.BP Kay Player Controller` null))

(event `self.OnHealthChanged`
  (params (DeltaBalue :type "Float (single-precision)") (EventTags :type "GameplayTagContainer Structure (by ref)"))
  (`self.UpdateHealthBar`))

(event `self.OnManaChanged`
  (params (DeltaBalue :type "Float (single-precision)") (EventTags :type "GameplayTagContainer Structure (by ref)"))
  (`self.UpdateManaBar`))

(fn `GetHealthInPercent`
  (returns (Percent :type "Float (double-precision)"))
  (`KismetSystemLibrary.PrintString` (`KismetStringLibrary.Conv_DoubleToString` (`self.GetHealth`)))
  (`KismetSystemLibrary.PrintString` (`KismetStringLibrary.Conv_DoubleToString` (`self.GetMaxHealth`)))
  (return 0.0))

(fn `UpdateHealthBar`)

(fn `UpdateManaBar`)

(fn `UserConstructionScript`
  (`parent.UserConstructionScript`))