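; Dungeon monster character Blueprint that reacts to health changes, damage, death and sight of the player.
; Health changes update its HP widget as a fraction of max health, while damage plays a hit montage and snaps the monster to face the instigator.
; AI perception writes whether a KayCharacter is sensed into the CanSeePlayer blackboard key.
; Post-death destroys the actor, and ShowDamageAmount is an empty stub.
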(event `self.OnHealthChanged`
  (params (DeltaBalue :type "Float (single-precision)") (EventTags :type "GameplayTagContainer Structure (by ref)"))
  (bind _aswb_enemy_hp (cast `/Game/Dungeon/WB/WB_EnemyHP` (`WidgetComponent.GetUserWidgetObject` (`self.HPWidget`))))
  (`/Game/Dungeon/WB/WB_EnemyHP.SetHpProgress` _aswb_enemy_hp (/ (`self.GetHealth`) (`self.GetMaxHealth`))))

(event `self.OnDamaged`
  (params (DamageAmount :type "Float (single-precision)") (HitInfo :type "HitResult Structure (by ref)") (DamageTags :type "GameplayTagContainer Structure (by ref)") (InstigatorCharacter :type "KayCharacter Object Reference") (DamageCauser :type "Actor Object Reference"))
  (`self.PlayAnimMontage` (`self.HitMontage`) 0.7)
  (`self.K2_SetActorRotation` (`KismetMathLibrary.FindLookAtRotation` (`self.K2_GetActorLocation`) (`self.K2_GetActorLocation` InstigatorCharacter))))

(event `self.OnPostDeath`
  (`self.K2_DestroyActor`))

(event `self.AIPerception.OnTargetPerceptionUpdated`
  (params (Actor :type "Actor Object Reference") (Stimulus :type "AIStimulus Structure"))
  (cast `KayCharacter` Actor)
  (`BlackboardComponent.SetValueAsBool` (`AIBlueprintHelperLibrary.GetBlackboard` null) "CanSeePlayer" (`.bSuccessfullySensed` (break `AIStimulus` Stimulus))))

(fn `ShowDamageAmount`)

(fn `UserConstructionScript`
  (`parent.UserConstructionScript`))