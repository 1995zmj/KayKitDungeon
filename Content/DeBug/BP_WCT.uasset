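; BP_WCT is a debug-folder Blueprint that shows hit damage text at world positions using pooled components.
; PlayHitNumber takes the last pooled component or creates one, then moves it, unhides it, binds its finished event and starts the damage text.
; When the finished event fires, Recycle hides the component and returns it to the pool.
; Tick records the current pool size in Count.
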(event `self.ReceiveBeginPlay`)

(event `self.ReceiveTick`
  (params (DeltaSeconds :type "Float (single-precision)"))
  (set `self.Count` (`KismetArrayLibrary.Array_Length` (`self.Pools`))))

(event `PlayHitNumber`
  (params (WorldPos :type "Vector Structure"))
  (bind _wc (`self.GetWC`))
  (`SceneComponent.K2_SetWorldLocation` _wc WorldPos false false)
  (`SceneComponent.SetHiddenInGame` _wc false false)
  (add `/Game/Dungeon/WB/WC_DamageText.WCFinshed` _wc (delegate `CustomEvent_0`))
  (`/Game/Dungeon/WB/WC_DamageText.SetDamageText` _wc))

(event `CustomEvent_0`
  (params (WC :type "/Game/Dungeon/WB/WC_DamageText Object Reference"))
  (`self.Recycle` WC))

(fn `CreateWC`
  (returns (WC :type "/Game/Dungeon/WB/WC_DamageText Object Reference"))
  (bind _returnvalue (`AddComponent|NODE_AddWC_DamageText-2`))
  (return _returnvalue))

(fn `GetWC`
  (returns (WC :type "/Game/Dungeon/WB/WC_DamageText Object Reference"))
  (locals (TempWC :type "/Game/Dungeon/WB/WC_DamageText Object Reference") (Index :type Integer))
  (bind _output_get (set `local.Index` (`KismetArrayLibrary.Array_Length` (`self.Pools`))))
  (if (> _output_get 0)
    (set `local.TempWC` (`|GetArrayItem` (`self.Pools`) (- (`local.Index`) 1)))
    (`KismetArrayLibrary.Array_Remove` (`self.Pools`) (- (`local.Index`) 1))
    (else
      (bind _wc (`self.CreateWC`))
      (set `local.TempWC` _wc)))
  (return (`local.TempWC`)))

(fn `Recycle`
  (params (WC :type "/Game/Dungeon/WB/WC_DamageText Object Reference"))
  (`SceneComponent.SetHiddenInGame` WC true false)
  (`KismetArrayLibrary.Array_Add` (`self.Pools`) WC))

(fn `UserConstructionScript`)